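; Rotating trap actor that a player arms by staying close, then damages surrounding non-player actors.
; Each tick, a small sphere trace looks for PlayerChar, sinking the trap and counting per hit, or resetting both when none is found.
; Past the count threshold, it spawns an effect, applies heavy damage to non-player hits in a much wider sphere trace, and destroys itself after a delay.
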(event Custom|MoveDown
  (bind _returnvalue (Transformation|GetActorLocation))
  (if (not (Variables|Default|GetIsTurn))
    (Transformation|AddWorldOffset (Variables|Default|GetDefaultSceneRoot) "0, 0,-0.100000" false false)
    (Variables|Default|SetFrame (+ (Variables|Default|GetFrame) 1))
    (if (> (Variables|Default|GetFrame) 100)
      (Variables|Default|SetIsTurn true)
      (Niagara|SpawnSystematLocation "/Game/Niagara/TrapTurnOnEmitter_System.TrapTurnOnEmitter_System" _returnvalue)
      (bind _outhits (Collision|MultiSphereTraceForObjects _returnvalue (+ _returnvalue 1.0) 2e+03 (Variables|Default|GetObject%20Types) false 0 "None"))
      (bind _array_element (Utilities|Array|ForEachLoopwithBreak _outhits)
        (:LoopBody
          (Utilities|Casting|CastToPlayerChar (.HitActor (Collision|BreakHitResult _array_element))
            (:CastFailed
              (Game|Damage|ApplyDamage (.HitActor (Collision|BreakHitResult _array_element)) 1e+03 0 0))))
        (:Completed
          (Utilities|FlowControl|Delay 2.0)
          (Actor|DestroyActor))))))

(event EventBeginPlay
  (Variables|Default|SetInitialLocation (Transformation|GetActorLocation)))

(event Collision|EventActorBeginOverlap
  (params (OtherActor :type Actor%20Object%20Reference)))

(event EventTick
  (params (DeltaSeconds :type Float%20%28single-precision%29))
  (bind _cylinder (Variables|Default|GetCylinder))
  (bind _returnvalue (Transformation|GetWorldLocation _cylinder))
  (Transformation|AddActorLocalRotation "0.000000,0.100000, 0" false false)
  (if (not (Variables|Default|GetIsTurn))
    (Variables|Default|SetHavePlayer false)
    (bind _outhits (Collision|MultiSphereTraceForObjects _returnvalue (+ _returnvalue 1.0) 2.5e+02 (Variables|Default|GetObject%20Types) false 0 "None"))
    (bind _array_element (Utilities|Array|ForEachLoopwithBreak _outhits)
      (:LoopBody
        (Utilities|Casting|CastToPlayerChar (.HitActor (Collision|BreakHitResult _array_element)))
        (Variables|Default|SetHavePlayer true)
        (CallFunction|MoveDown))
      (:Completed
        (if (not (Variables|Default|GetHavePlayer))
          (Variables|Default|SetFrame 0)
          (Transformation|SetActorLocation (Variables|Default|GetInitialLocation) false false))))))

(fn ConstructionScript)